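; Enemy character with melee axe and area attacks, an overhead-style health widget fed by BPCStats, and ragdoll death.
; Damage lowers the stat and plays a hit-react montage that halts movement; interactor overlaps toggle the widget.
; Attack functions play montages and sounds, while separate events run a timer-looped, cooldown-gated axe sphere trace or a one-shot point trace with explosion, sound and camera shake.
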(event OnComponentBeginOverlap(Trigger)
  (params (OverlappedComponent :type Primitive%20Component%20Object%20Reference) (OtherActor :type Actor%20Object%20Reference) (OtherComp :type Primitive%20Component%20Object%20Reference) (OtherBodyIndex :type Integer) (bFromSweep :type Boolean) (SweepResult :type Hit%20Result%20Structure%20%28by%20ref%29))
  (if (Utilities|DoesObjectImplementInterface OtherActor "/Game/Blueprints/Weapons/BPI_Interact.BPI_Interact_C")
    (Rendering|SetVisibility (Variables|Default|GetWidget) true false)))

(event OnComponentEndOverlap(Trigger)
  (params (OverlappedComponent :type Primitive%20Component%20Object%20Reference) (OtherActor :type Actor%20Object%20Reference) (OtherComp :type Primitive%20Component%20Object%20Reference) (OtherBodyIndex :type Integer))
  (if (Utilities|DoesObjectImplementInterface OtherActor "/Game/Blueprints/Weapons/BPI_Interact.BPI_Interact_C")
    (Rendering|SetVisibility (Variables|Default|GetWidget) false false)))

(event Custom|Damage%20Trace
  ;[0.15 0.15 0.15 0.5] Axe Traces
  (if (not (Variables|Default|GetisDead?))
    (bind _outhit (Collision|SphereTraceForObjects (Transformation|GetWorldLocation (Variables|Default|GetStart%20Axe%20Trace%20Pos)) (Transformation|GetWorldLocation (Variables|Default|GetEnd%20Axe%20Trace%20Pos)) (Variables|Default|GetswordAttackRadius) (Utilities|Array|MakeArray "ObjectTypeQuery3") false 0 "ForOneFrame"))
    (if true
      (Utilities|FlowControl|DoOnce false :!label _label
        (:Completed
          (Game|Damage|ApplyDamage (.HitActor (Collision|BreakHitResult _outhit)) (Variables|Default|GetaxeDamage) 0 0)
          (Utilities|FlowControl|Delay 0.3)
          (goto _label Reset))))))

(event EventBeginAxeTrace
  ;[0.15 0.15 0.15 0.5] Axe Traces
  (bind _returnvalue (Utilities|Time|SetTimerbyEvent (delegate Custom|Damage%20Trace) 0.01 true)))

(event EventEndAxeTrace
  ;[0.15 0.15 0.15 0.5] Axe Traces
  (if (Utilities|Time|IsValidTimerHandle (stale EventBeginAxeTrace _returnvalue))
    (Utilities|Time|ClearandInvalidateTimerbyHandle (stale EventBeginAxeTrace _returnvalue))))

(event EventBeginPlay
  (bind _aswb_enemy_health (Utilities|Casting|CastToWB_EnemyHealth (UserInterface|GetWidget (Variables|Default|GetWidget))))
  (Default|SetHealthProgressBar (Variables|Default|GetBPC_Stats) (Variables|/Game/UI/WB_EnemyHealth.WB_EnemyHealth_C|GetHealthBar _aswb_enemy_health))
  (Components|SkinnedMesh|HideBonebyName (Variables|Default|GetAchilles) "Shield_joint" "PBO_None")
  (Variables|Default|SetinitialWalkSpeed (Variables|/Script/Engine.CharacterMovementComponent|GetMaxWalkSpeed (Variables|Character|GetCharacterMovement))))

(event Game|Damage|EventAnyDamage
  (params (Damage :type Float%20%28single-precision%29) (DamageType :type Damage%20Type%20Object%20Reference) (InstigatedBy :type Controller%20Object%20Reference) (DamageCauser :type Actor%20Object%20Reference))
  (Default|IncreaseValue (Variables|Default|GetBPC_Stats) "NewEnumerator0" (* Damage -1.0))
  (Animation|Montage|PlayMontage (Variables|Character|GetMesh) "/Game/Characters/Souls/Combat/HitReact_Montage.HitReact_Montage"
    (:then
      (Variables|/Script/Engine.CharacterMovementComponent|SetMaxWalkSpeed (Variables|Character|GetCharacterMovement) 0.0))
    (:OnCompleted
      (Variables|/Script/Engine.CharacterMovementComponent|SetMaxWalkSpeed (Variables|Character|GetCharacterMovement) (Variables|Default|GetinitialWalkSpeed) :!label _label))
    (:OnInterrupted
      (goto _label))))

(event EventDie
  (Pawn|Components|CharacterMovement|DisableMovement (Variables|Character|GetCharacterMovement))
  (Physics|SetSimulatePhysics (Variables|Character|GetMesh) true)
  (Variables|Default|SetisDead? true))

(event EventPointDamageTrace
  (bind _point_trace_pos (Variables|Default|GetPoint%20Trace%20Pos))
  (bind _point_trace_pos_2 (Variables|Default|GetPoint%20Trace%20Pos))
  (bind _returnvalue (Transformation|GetWorldLocation _point_trace_pos))
  (bind _returnvalue_2 (Transformation|GetWorldLocation _point_trace_pos_2))
  (Utilities|FlowControl|Sequence
    (:then_0
      (if (not (Variables|Default|GetisDead?))
        (bind (_outhit _returnvalue_3) (Collision|SphereTraceForObjects _returnvalue_2 _returnvalue_2 (Variables|Default|GetpointAttackRadius) (Utilities|Array|MakeArray "ObjectTypeQuery3") false 0 "ForDuration" true "(R=1.000000,G=0.000000,B=0.000000,A=1.000000)" "(R=0.000000,G=1.000000,B=0.000000,A=1.000000)" 1.0))
        (if _returnvalue_3
          (Game|Damage|ApplyDamage (.HitActor (Collision|BreakHitResult _outhit)) 2e+01 0 0))))
    (:then_1
      (Audio|PlaySoundatLocation "/Game/Audio/Sounds/SC_Stomp.SC_Stomp" _returnvalue "0, 0, 0" 1.0 1.0 0.0 0 0 0 0)
      (Camera|PlayWorldCameraShake "/Game/Blueprints/BP_CameraShake_Attack.BP_CameraShake_Attack_C" _returnvalue 0.0 2e+03)
      (Effects|SpawnEmitteratLocation "/Game/StarterContent/Particles/P_Explosion.P_Explosion" _returnvalue "0, 0, 0" "1.000000,1.000000,1.000000" true "AutoRelease"))))

(fn ConstructionScript)

(fn BigAttack
  (bind _returnvalue (Animation|PlayAnimMontage (Variables|Default|GetbigAttackMontage) 1.0 "None"))
  (Audio|PlaySoundatLocation "/Game/Audio/Sounds/SC_Stomp.SC_Stomp" (Transformation|GetActorLocation) "0, 0, 0" 1.0 1.0 0.0 0 0 0 0)
  (return _returnvalue))

(fn SwordAttack
  (bind _returnvalue (Animation|PlayAnimMontage (Variables|Default|GetswordAttackMontage) 1.0 "None"))
  (Audio|PlaySoundatLocation (Variables|Default|GetSword%20Attack%20Sound) (Transformation|GetActorLocation) "0, 0, 0" 1.0 1.0 0.0 0 0 0 0)
  (return _returnvalue))